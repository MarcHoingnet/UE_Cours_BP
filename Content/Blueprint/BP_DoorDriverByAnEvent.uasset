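; Door actor that toggles between two positions whenever a referenced EventLuncher fires its ActivateControllables event dispatcher.
; On BeginPlay it binds ActivationDoor to that dispatcher, and that event calls ToggleDoor.
; ToggleDoor checks the Cube's relative X and snaps it between the origin and an X offset, with no sweep or animation.
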(event Custom|ActivationDoor
  (CallFunction|ToggleDoor))

(event EventBeginPlay
  (EventDispatchers|BindEventtoActivateControllables (Variables|Default|GetEventLuncher) (delegate Custom|ActivationDoor)))

(fn ConstructionScript)

(fn ToggleDoor
  (bind _cube (Variables|Default|GetCube))
  (if (> (.x (Variables|/Script/Engine.SceneComponent|GetRelativeLocation (Variables|Default|GetCube))) 0.0)
    (Transformation|SetRelativeLocation _cube "0, 0, 0" false false)
    (else
      (Transformation|SetRelativeLocation _cube "100.000000,0.000000,0.000000" false false))))